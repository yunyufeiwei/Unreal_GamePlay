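; BP_C_Character is a player character Blueprint that handles basic keyboard and mouse movement, look and jump through Enhanced Input.
; On BeginPlay it adds the keyboard/mouse mapping context to the owning player controller's input subsystem.
; Move input is applied along forward and right vectors from player 0's control yaw, keeping movement camera-relative and horizontal.
; Mouse look feeds controller yaw and pitch, and the jump action calls Jump.
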(event Input|EnhancedActionEvents|EnhancedInputActionIA_Move
  (params (ActionValue :type Vector%202D%20Structure) (ElapsedSeconds :type Float%20%28double-precision%29) (TriggeredSeconds :type Float%20%28double-precision%29) (InputAction :type Input%20Action%20Object%20Reference :default "/Game/PlayerMovement/Input/Action/IA_Move.IA_Move"))
  (bind _returnvalue (Game|GetPlayerController 0))
  (bind (_x _y) (Math|Vector2D|BreakVector2D ActionValue))
  (bind _returnvalue_2 (Pawn|GetControlRotation _returnvalue :!class /Script/Engine.Controller))
  (bind _yaw (Math|Rotator|BreakRotator _returnvalue_2))
  (bind _returnvalue_3 (Math|Rotator|MakeRotator 0.0 0.0 _yaw))
  ;[1 1 1] Kyeboard
  (:Triggered
    (Pawn|Input|AddMovementInput (Math|Vector|GetForwardVector _returnvalue_3) _y false)
    (Pawn|Input|AddMovementInput (Math|Vector|GetRightVector _returnvalue_3) _x false)))

(event Input|EnhancedActionEvents|EnhancedInputActionIA_Look_Mouse
  (params (ActionValue :type Vector%202D%20Structure) (ElapsedSeconds :type Float%20%28double-precision%29) (TriggeredSeconds :type Float%20%28double-precision%29) (InputAction :type Input%20Action%20Object%20Reference :default "/Game/PlayerMovement/Input/Action/IA_Look_Mouse.IA_Look_Mouse"))
  (bind (_x _y) (Math|Vector2D|BreakVector2D ActionValue))
  ;[1 1 1] Mosue
  (:Triggered
    (Pawn|Input|AddControllerYawInput _x)
    (Pawn|Input|AddControllerPitchInput _y)))

(event Input|EnhancedActionEvents|EnhancedInputActionIA_Jump
  (params (ActionValue :type Boolean) (ElapsedSeconds :type Float%20%28double-precision%29) (TriggeredSeconds :type Float%20%28double-precision%29) (InputAction :type Input%20Action%20Object%20Reference :default "/Game/PlayerMovement/Input/Action/IA_Jump.IA_Jump"))
  (:Triggered
    (Character|Jump)))

(event EventBeginPlay
  ;[1 1 1] 输入映射上下文
  (bind _asplayer_controller (Utilities|Casting|CastToPlayerController (Pawn|GetController)))
  (Utilities|IsValid (PlayerController|LocalPlayerSubsystems|GetEnhancedInputLocalPlayerSubsystem _asplayer_controller)
    (:Is%20Valid
      (Input|AddMappingContext (PlayerController|LocalPlayerSubsystems|GetEnhancedInputLocalPlayerSubsystem _asplayer_controller) "/Game/PlayerMovement/Input/Configs/IMC_Default_KBM.IMC_Default_KBM" 0 "(bIgnoreAllPressedKeysUntilRelease=True,bForceImmediately=False)"))))

(fn ConstructionScript)